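; MonsterSpawn_2 is a monster actor that repeatedly appears and disappears on a timer by toggling its visibility, without spawning anything.
; Shortly after BeginPlay it hides itself, then loops: wait MonsterSpawnTime, show, wait MonsterExistTIme, hide.
; The IsHidden flag gates each step and runs inverted, true while visible, so the cycle starts only if it is true at BeginPlay.
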(event `self.ReceiveBeginPlay`
  ;[1 1 1] At start Hide Monster
  (`KismetSystemLibrary.Delay` 0.4)
  (if (`self.IsHidden?`)
    (`self.SetActorHiddenInGame` true)
    (set `self.IsHidden?` false)
    ;[1 1 1] Monster Visible
    (`KismetSystemLibrary.Delay` (`self.MonsterSpawnTime`) :!label _label)
    (if (not (`self.IsHidden?`))
      (`self.SetActorHiddenInGame` false)
      (set `self.IsHidden?` true)
      ;[1 1 1] Monster to Invisible
      (`KismetSystemLibrary.Delay` (`self.MonsterExistTIme`))
      (if (`self.IsHidden?`)
        (`self.SetActorHiddenInGame` true)
        (set `self.IsHidden?` false)
        (goto _label)))))

(fn `UserConstructionScript`)