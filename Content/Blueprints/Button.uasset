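; Pressure button Blueprint whose mesh sinks while any actor overlaps its Box and rises back when the Box is clear.
; Tick polls the overlap and shifts the height by a fixed step per frame through near-instant MoveComponentTo calls, clamped between zero and ButtonOffset.
; The construction script uses ButtonOffset to set the mesh's raised position and the Arrow's length.
; It only handles the motion and triggers nothing else.
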(event `self.ReceiveTick`
  (params (DeltaSeconds :type "Float (single-precision)"))
  (bind _staticmesh (`self.StaticMesh`))
  (bind (_relativelocation_x _relativelocation_y _relativelocation_z) (`KismetMathLibrary.BreakVector` (`SceneComponent.RelativeLocation` (`self.StaticMesh`))))
  (bind (_relativelocation_x_2 _relativelocation_y_2 _relativelocation_z_2) (`KismetMathLibrary.BreakVector` (`SceneComponent.RelativeLocation` _staticmesh)))
  (if (> (`KismetArrayLibrary.Array_Length` (`PrimitiveComponent.GetOverlappingActors` (`self.Box`) null)) 0)
    (`KismetSystemLibrary.MoveComponentTo` _staticmesh (`KismetMathLibrary.MakeVector` 0.0 0.0 (`KismetMathLibrary.FClamp` (- _relativelocation_z_2 3.0) 0.0 (`self.ButtonOffset`))) (struct) false false 1e-05)
    (else
      (`KismetSystemLibrary.MoveComponentTo` null (`KismetMathLibrary.MakeVector` 0.0 0.0 (`KismetMathLibrary.FClamp` (+ _relativelocation_z 3.0) 0.0 (`self.ButtonOffset`))) (struct) false false 1e-05))))

(fn `UserConstructionScript`
  (bind _buttonoffset (`self.ButtonOffset`))
  (set `ArrowComponent.ArrowLength` _buttonoffset (`self.Arrow`))
  (`SceneComponent.K2_SetRelativeLocation` (`self.StaticMesh`) (`KismetMathLibrary.MakeVector` 0.0 0.0 _buttonoffset) false false))